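; BP_LK_DoorReset is a door that opens when the player is not facing it, by hiding its mesh and disabling collision.
; Each Tick it opens only if the actor location fails to project to screen and the player overlaps LookAtTrigger; otherwise it closes.
; While it is open, a player overlapping ClearanceTrigger destroys the actor, removing the door permanently.
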(event `self.ReceiveTick`
  (params (DeltaSeconds :type "Float (single-precision)"))
  (bind _staticmeshcomponent (`self.StaticMeshComponent`))
  (bind _staticmeshcomponent_2 (`self.StaticMeshComponent`))
  (if (and (not (`.ReturnValue` (`PlayerController.ProjectWorldLocationToScreen` (`GameplayStatics.GetPlayerController` 0) (`self.K2_GetActorLocation`) false))) (`self.IsOverlappingActor` (`self.LookAtTrigger`) (`GameplayStatics.GetPlayerCharacter` 0)))
    ;[1 1 1] Open
    (`PrimitiveComponent.SetCollisionEnabled` _staticmeshcomponent_2 "NoCollision")
    (`SceneComponent.SetHiddenInGame` _staticmeshcomponent_2 true false)
    (if (`PrimitiveComponent.IsOverlappingActor` (`self.ClearanceTrigger`) (`GameplayStatics.GetPlayerCharacter` 0))
      (`self.K2_DestroyActor`))
    (else
      ;[1 1 1] Close
      (`PrimitiveComponent.SetCollisionEnabled` _staticmeshcomponent "QueryAndPhysics")
      (`SceneComponent.SetHiddenInGame` _staticmeshcomponent false false))))

(fn `UserConstructionScript`)