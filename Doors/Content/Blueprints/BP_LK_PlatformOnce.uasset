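; BP_LK_PlatformOnce is a platform that starts hidden without collision and appears permanently once the player is nearby and not facing it.
; Each Tick reveals it when the player overlaps ProximityTrigger, is outside ClearanceTrigger, and the actor's location fails screen projection.
; The projection check uses only the success flag, not viewport bounds, so it effectively requires the actor's origin to be behind the camera.
; Nothing hides the platform again.
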(event `self.ReceiveBeginPlay`
  (bind _platform (`self.Platform`))
  (`PrimitiveComponent.SetCollisionEnabled` _platform "NoCollision")
  (`SceneComponent.SetHiddenInGame` _platform true false))

(event `self.ReceiveTick`
  (params (DeltaSeconds :type "Float (single-precision)"))
  (bind _platform (`self.Platform`))
  (if (and (not (`.ReturnValue` (`PlayerController.ProjectWorldLocationToScreen` (`GameplayStatics.GetPlayerController` 0) (`self.K2_GetActorLocation`) false))) (`PrimitiveComponent.IsOverlappingActor` (`self.ProximityTrigger`) (`GameplayStatics.GetPlayerCharacter` 0)) (not (`PrimitiveComponent.IsOverlappingActor` (`self.ClearanceTrigger`) (`GameplayStatics.GetPlayerCharacter` 0))))
    (`PrimitiveComponent.SetCollisionEnabled` _platform "QueryAndPhysics")
    (`SceneComponent.SetHiddenInGame` _platform false false)))

(fn `UserConstructionScript`)