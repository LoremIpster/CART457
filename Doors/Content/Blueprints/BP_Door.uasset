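; BP_Door is a door that swings open on a scripted timeline, then hands over to physics simulation.
; StartWithPhysics sets whether the door simulates physics from BeginPlay.
; The Open event plays a timeline that lerps from the door's current rotation toward a fixed angle, enabling physics when finished.
; Any overlap with the Trigger component stops the timeline and switches physics on immediately.
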(event `self.ReceiveBeginPlay`
  (bind _door (`self.Door`))
  (if (`self.startWithPhysics`)
    (`PrimitiveComponent.SetSimulatePhysics` _door true)
    (else
      (`PrimitiveComponent.SetSimulatePhysics` _door false))))

(event `Open`
  (bind _door (`self.Door`))
  (bind (_direction _open) (`Timeline|Timeline_0` :!label _label)
    (:`Update`
      (`SceneComponent.K2_SetRelativeRotation` _door (`KismetMathLibrary.RLerp` (`SceneComponent.RelativeRotation` _door) (struct :`Yaw` -50.0) _open true) false false))
    (:`Finished`
      (`PrimitiveComponent.SetSimulatePhysics` _door true :!label _label_2))))

(event `self.Trigger.OnComponentBeginOverlap`
  (params (OverlappedComponent :type "PrimitiveComponent Object Reference") (OtherActor :type "Actor Object Reference") (OtherComp :type "PrimitiveComponent Object Reference") (OtherBodyIndex :type Integer) (bFromSweep :type Boolean) (SweepResult :type "HitResult Structure (by ref)"))
  (`|ExecutionSequence`
    (:`then_0`
      (goto _label :!via `Stop`))
    (:`then_1`
      (goto _label_2))))

(fn `UserConstructionScript`)