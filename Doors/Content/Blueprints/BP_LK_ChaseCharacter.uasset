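; BP_LK_ChaseCharacter is a chasing character that advances on the player only while unobserved.
; Being looked at stops its movement and sets HasBeenSeen, which arms the chase.
; Once armed, the not-looking event uses SimpleMoveToActor toward the player pawn.
; The KillRadius overlap event is empty; the cast and Death call on FirstPersonCharacter are disconnected and never run.
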(event `PlayerIsNotLooking`
  (if (`self.HasBeenSeen`)
    (`NavigationSystem.SimpleMoveToActor` (`self.GetController`) (`GameplayStatics.GetPlayerPawn` 0))))

(event `PlayerIsLooking`
  (`Controller.StopMovement` (`self.GetController`))
  (if (not (`self.HasBeenSeen`))
    (set `self.HasBeenSeen` true)))

(event `self.KillRadius.OnComponentBeginOverlap`
  (params (OverlappedComponent :type "PrimitiveComponent Object Reference") (OtherActor :type "Actor Object Reference") (OtherComp :type "PrimitiveComponent Object Reference") (OtherBodyIndex :type Integer) (bFromSweep :type Boolean) (SweepResult :type "HitResult Structure (by ref)")))

(fn `UserConstructionScript`)